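; BP_Spawner is an actor that periodically spawns enemies of a configured class, keeping the live count under a maximum.
; Tick counts down a randomized cooldown, then requests a point within a radius from the level's BP_SpawnSystem, which BeginPlay requires to exist.
; Each enemy spawns facing the player pawn, and its OnDie event is bound, apparently to decrement the count and free a slot.
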(event `self.ReceiveBeginPlay`
  (bind _returnvalue (`GameplayStatics.GetActorOfClass` "/Game/Content/Game/Spawn/BP_SpawnSystem.BP_SpawnSystem_C"))
  (bind _output_get (set `self.SpawnSystem` _returnvalue))
  (`/Engine/EditorBlueprintResources/StandardMacros.IsValid` _output_get
    (:`Is Valid`
      _)
    (:`Is Not Valid`
      (`KismetSystemLibrary.RaiseScriptError` "Place BP_SpawnSystem in the level")))
  (`self.RefreshSpawnTimer`))

(event `self.ReceiveTick`
  (params (DeltaSeconds :type "Float (single-precision)"))
  (bind _output_get (set `self.SpawnTimer` (- (`self.SpawnTimer`) DeltaSeconds)))
  (if (<= _output_get 0.0)
    (`self.SpawnEnemy`)
    (`self.RefreshSpawnTimer`)))

(event `OnSpawnedEnemyDied`
  (`/Engine/EditorBlueprintResources/StandardMacros.DecrementInt` (`self.EnemiesCount`)))

(fn `RefreshSpawnTimer`
  (bind (_spawncooldown_min _spawncooldown_max) (break `FloatInterval` (`self.SpawnCooldown`)))
  (set `self.SpawnTimer` (`KismetMathLibrary.RandomFloatInRange` _spawncooldown_min _spawncooldown_max)))

(fn `SpawnEnemy`
  (if (< (`self.EnemiesCount`) (`self.MaxEnemiesCount`))
    (bind (_randomlocation _success) (`/Game/Content/Game/Spawn/BP_SpawnSystem.GetSpawnPointAround` (`self.SpawnSystem`) (`self.SpawnAroundActor`) (`self.SpawnCenter`) (`self.SpawnRadius`)))
    (if _success
      (bind _returnvalue (`|SpawnActorFromClass` (`self.EnemyClass`) (`KismetMathLibrary.MakeTransform` _randomlocation (`KismetMathLibrary.FindLookAtRotation` _randomlocation (`self.K2_GetActorLocation` (`GameplayStatics.GetPlayerPawn` 0)))) "Undefined" "MultiplyWithRoot" null 1 100.0 1.0 null))
      (add `/Game/AI/BP_EnemyBasic.OnDie` _returnvalue (`|CreateDelegate` :!event `OnSpawnedEnemyDied`))
      (`/Engine/EditorBlueprintResources/StandardMacros.IncrementInt` (`self.EnemiesCount`)))))

(fn `UserConstructionScript`)