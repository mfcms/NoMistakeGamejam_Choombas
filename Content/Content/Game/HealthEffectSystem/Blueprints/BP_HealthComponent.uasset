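; Health component that tracks an owner's current health and death state.
; HandleDamage scales incoming damage by a per-damage-type multiplier map, defaulting to unscaled, then clamps health between zero and the maximum.
; When health reaches zero, Die sets a guard flag and fires the OnDeath dispatcher only once.
; GetHealthForHUD exposes current and maximum health for display.
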(fn `Die`
  (if (not (`self.bDead`))
    (set `self.bDead` true)
    (`self.OnDeath`)))

(fn `GetHealthForHUD`
  (returns (Current :type "Float (double-precision)") (Maximum :type "Float (double-precision)"))
  (return (`self.CurrentHealth`) (`self.MaxHealth`)))

(fn `HandleDamage`
  (params (BaseDamage :type "Float (double-precision)") (DamageType :type "/Game/Content/Game/HealthEffectSystem/Enums/E_DamageType Enum" :default "NewEnumerator4") (DamageCauser :type "Actor Object Reference"))
  (locals (Multiplier :type "Float (double-precision)"))
  (bind (_value _returnvalue) (`BlueprintMapLibrary.Map_Find` (`self.DamageMultipliers`) DamageType))
  (if _returnvalue
    (set `local.Multiplier` _value)
    (else
      (set `local.Multiplier` 1.0)))
  (bind _output_get (set `self.CurrentHealth` (`KismetMathLibrary.FClamp` (- (`self.CurrentHealth`) (* BaseDamage (`local.Multiplier`))) 0.0 (`self.MaxHealth`))))
  (if (<= _output_get 0.0)
    (`self.Die`)))