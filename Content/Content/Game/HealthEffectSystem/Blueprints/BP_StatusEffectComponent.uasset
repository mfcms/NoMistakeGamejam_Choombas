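; Actor component that manages timed or infinite status effects (Stunned, Burning, Slowed) on its owner, stored in a map by type.
; Reapplying an effect keeps the later expiry and takes the new magnitude and interval.
; One timer, rescheduled to the nearest expiry, drives removal instead of Tick.
; Stun toggles CanAct and broadcasts changes, Burning deals looping fire damage, and Slowed scales the Character's base walk speed.
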(event EventBeginPlay
  (bind _ascharacter (Utilities|Casting|CastToCharacter (Components|GetOwner)))
  (Variables|/Script/Engine.CharacterMovementComponent|SetMaxWalkSpeed (Variables|/Script/Engine.Character|GetCharacterMovement _ascharacter) (Variables|Default|GetBaseWalkSpeed)))

(event EventTick
  (params (DeltaSeconds :type Float%20%28single-precision%29)))

(fn HasStatusEffect
  (params (Type :type E_StatusEffect%20Enum :default "NewEnumerator0"))
  (bind _activeeffects (Variables|Default|GetActiveEffects))
  (bind (_value _returnvalue) (Utilities|Map|Find _activeeffects Type))
  (return _returnvalue _value))

(fn RecalculateCanAct
  (bind _haseffect (CallFunction|HasStatusEffect "NewEnumerator2"))
  (if (!= (not _haseffect) (Variables|Default|GetbCanAct))
    (bind _output_get (Variables|Default|SetbCanAct (not _haseffect)))
    (Default|CallOnCanActChanged _output_get)))

(fn ApplyStatusEffect
  (params (Type :type E_StatusEffect%20Enum :default "NewEnumerator0") (Duration :type Float%20%28double-precision%29) (Infifnite :type Boolean) (Magnitude :type Float%20%28double-precision%29) (TickInterval :type Float%20%28double-precision%29))
  (LocalVariables|SetResultStatusEffect (Utilities|Struct|MakeST_ActiveStatusEffect Type (+ Duration (Utilities|Time|GetGameTimeinSeconds)) Infifnite Magnitude TickInterval))
  (bind (_haseffect _activestatuseffect) (CallFunction|HasStatusEffect Type))
  (if _haseffect
    (LocalVariables|SetResultStatusEffect (Utilities|Struct|MakeST_ActiveStatusEffect (.Type (Utilities|Struct|BreakST_ActiveStatusEffect _activestatuseffect)) (Math|Float|Max(Float) (.ExpireAt (Utilities|Struct|BreakST_ActiveStatusEffect _activestatuseffect)) (+ Duration (Utilities|Time|GetGameTimeinSeconds))) (or (.bInfinite (Utilities|Struct|BreakST_ActiveStatusEffect _activestatuseffect)) Infifnite) (.magnitude (LocalVariables|GetResultStatusEffect)) (.tickinterval (LocalVariables|GetResultStatusEffect)))))
  (Utilities|Map|Add (Variables|Default|GetActiveEffects) (.type (LocalVariables|GetResultStatusEffect)) (LocalVariables|GetResultStatusEffect))
  (CallFunction|RecalculateCanAct)
  (CallFunction|ScheduleNextStatusExpiration)
  (switch Utilities|FlowControl|Switch|SwitchonE_StatusEffect (.type (LocalVariables|GetResultStatusEffect))
    (:NewEnumerator0
      (CallFunction|StartBurning))
    (:NewEnumerator3
      (CallFunction|RecalculateMovementSpeed))))

(fn RemoveStatusEffect
  (params (Type :type E_StatusEffect%20Enum :default "NewEnumerator0"))
  (bind (_haseffect _activestatuseffect) (CallFunction|HasStatusEffect Type))
  (if _haseffect
    (Utilities|Map|Remove (Variables|Default|GetActiveEffects) (.type _activestatuseffect))
    (CallFunction|RecalculateCanAct)
    (CallFunction|ScheduleNextStatusExpiration)))

(fn ScheduleNextStatusExpiration
  (LocalVariables|SetbFoundExpiration false)
  (Utilities|Time|ClearandInvalidateTimerbyHandle (Variables|Default|GetStatusExpirationTimer))
  (bind _valuepin (Utilities|Map|ForEachLoop(Map) (Variables|Default|GetActiveEffects))
    (:then
      (if (not (.bInfinite (Utilities|Struct|BreakST_ActiveStatusEffect _valuepin)))
        (if (LocalVariables|GetbFoundExpiration)
          (if (< (.ExpireAt (Utilities|Struct|BreakST_ActiveStatusEffect _valuepin)) (LocalVariables|GetNearestExpireAt))
            (LocalVariables|SetNearestExpireAt (.ExpireAt (Utilities|Struct|BreakST_ActiveStatusEffect _valuepin))))
          (else
            (LocalVariables|SetNearestExpireAt (.ExpireAt (Utilities|Struct|BreakST_ActiveStatusEffect _valuepin)))
            (LocalVariables|SetbFoundExpiration true)))))
    (:CompletedPin
      (if (LocalVariables|GetbFoundExpiration)
        (bind _output_get (LocalVariables|SetDelay (|(max(({CBF0877D-4D86-F1F7-4E69-D1AD24D1341D}-now),0.010000)) (Utilities|Time|GetGameTimeinSeconds))))
        (bind _returnvalue (Utilities|Time|SetTimerbyEvent (EventDispatchers|CreateEvent :!event ProcessExpiredStatuses) _output_get))
        (Variables|Default|SetStatusExpirationTimer _returnvalue)))))

(fn ProcessExpiredStatuses
  (bind _activeeffects (Variables|Default|GetActiveEffects))
  (bind _keys (Utilities|Map|Keys _activeeffects))
  (for _array_element _keys
    (if (.ReturnValue (Utilities|Map|Find _activeeffects _array_element))
      (if (and (not (.bInfinite (Utilities|Struct|BreakST_ActiveStatusEffect (.Value (Utilities|Map|Find _activeeffects _array_element))))) (<= (.ExpireAt (Utilities|Struct|BreakST_ActiveStatusEffect (.Value (Utilities|Map|Find _activeeffects _array_element)))) (Utilities|Time|GetGameTimeinSeconds)))
        (Utilities|Map|Remove _activeeffects _array_element)
        (switch Utilities|FlowControl|Switch|SwitchonE_StatusEffect _array_element
          (:NewEnumerator3
            (CallFunction|RecalculateMovementSpeed))))))
  (CallFunction|RecalculateCanAct)
  (CallFunction|ScheduleNextStatusExpiration)
  (switch Utilities|FlowControl|Switch|SwitchonE_StatusEffect _array_element
    (:NewEnumerator3
      (CallFunction|RecalculateMovementSpeed))))

(fn StartBurning
  (bind (_haseffect _activestatuseffect) (CallFunction|HasStatusEffect "NewEnumerator0"))
  (if _haseffect
    (Utilities|Time|ClearandInvalidateTimerbyHandle (Variables|Default|GetBurningTimerHandle))
    (bind _returnvalue (Utilities|Time|SetTimerbyFunctionName 0 "BurningTick" (.TickInterval (Utilities|Struct|BreakST_ActiveStatusEffect _activestatuseffect)) true))
    (Variables|Default|SetBurningTimerHandle _returnvalue)))

(fn BurningTick
  (bind (_haseffect _activestatuseffect) (CallFunction|HasStatusEffect "NewEnumerator0"))
  (if _haseffect
    (Game|Damage|ApplyDamage (Components|GetOwner) (.Magnitude (Utilities|Struct|BreakST_ActiveStatusEffect _activestatuseffect)) 0 0 "/Game/Content/Game/HealthEffectSystem/Blueprints/BP_DT_Fire.BP_DT_Fire_C")
    (else
      (Utilities|Time|ClearandInvalidateTimerbyHandle (Variables|Default|GetBurningTimerHandle)))))

(fn RecalculateMovementSpeed
  (bind _basewalkspeed (Variables|Default|GetBaseWalkSpeed))
  (bind (_haseffect _activestatuseffect) (CallFunction|HasStatusEffect "NewEnumerator3"))
  (bind _ascharacter (Utilities|Casting|CastToCharacter (Components|GetOwner)))
  (if _haseffect
    (Variables|/Script/Engine.CharacterMovementComponent|SetMaxWalkSpeed (Variables|/Script/Engine.Character|GetCharacterMovement _ascharacter) (* _basewalkspeed (Math|Float|Clamp(Float) (.Magnitude (Utilities|Struct|BreakST_ActiveStatusEffect _activestatuseffect)) 0.05 1e+01)))
    (else
      (Variables|/Script/Engine.CharacterMovementComponent|SetMaxWalkSpeed (Variables|/Script/Engine.Character|GetCharacterMovement _ascharacter) _basewalkspeed))))

(fn SetDesiredWalkSpeed
  (params (NewSpeed :type Float%20%28double-precision%29))
  (Variables|Default|SetBaseWalkSpeed NewSpeed)
  (CallFunction|RecalculateMovementSpeed))

(fn GetConfiguredWalkSpeed
  (params (FallbackSpeed :type Float%20%28double-precision%29))
  (bind _maxspeedoverride (Variables|GD|GetMaxSpeedOverride))
  (return (Math|Float|SelectFloat _maxspeedoverride FallbackSpeed (> _maxspeedoverride 0.0))))