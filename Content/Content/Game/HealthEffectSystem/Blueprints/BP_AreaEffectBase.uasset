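; BP_AreaEffectBase is a timed area-effect actor that repeatedly applies a status effect to nearby actors.
; InitArea stores the area and status parameters, starts a looping AreaPulse timer and sets the actor's lifespan to the area duration.
; Each pulse applies the status through BP_StatusEffectComponent on every SphereCollision overlap except the caster.
; The Radius value is stored but not applied to the sphere in these graphs.
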(fn `AreaPulse`
  (for _array_element (`PrimitiveComponent.GetOverlappingActors` (`self.SphereCollision`) null)
    (if (!= _array_element (`self.Caster`))
      (bind _returnvalue (`self.GetComponentByClass` _array_element "/Game/Content/Game/HealthEffectSystem/Blueprints/BP_StatusEffectComponent.BP_StatusEffectComponent_C"))
      (if (`KismetSystemLibrary.IsValid` _returnvalue)
        (`/Game/Content/Game/HealthEffectSystem/Blueprints/BP_StatusEffectComponent.ApplyStatusEffect` _returnvalue (`self.StatusType`) (`self.StatusDuration`) (`self.StatusInfinite`) (`self.StatusMagnitude`) (`self.StatusTickInterval`))))))

(fn `InitArea`
  (params (Radius :type "Float (double-precision)") (AreaDuration :type "Float (double-precision)") (PulseInterval :type "Float (double-precision)") (StatusType :type "/Game/Content/Game/HealthEffectSystem/Enums/E_StatusEffect Enum" :default "NewEnumerator0") (StatusDuration :type "Float (double-precision)") (StatusMagnitude :type "Float (double-precision)") (StatusTickInterval :type "Float (double-precision)") (StatusInfinite :type Boolean) (Caster :type "Actor Object Reference"))
  (set `self.Radius` Radius)
  (set `self.AreaDuration` AreaDuration)
  (set `self.PulseInterval` PulseInterval)
  (set `self.StatusType` StatusType)
  (set `self.StatusDuration` StatusDuration)
  (set `self.StatusTickInterval` StatusTickInterval)
  (set `self.StatusMagnitude` StatusMagnitude)
  (set `self.StatusInfinite` StatusInfinite)
  (set `self.Caster` Caster)
  (bind _returnvalue (`KismetSystemLibrary.K2_SetTimer` null "AreaPulse" (`self.PulseInterval`) true))
  (set `self.EffectTimer` _returnvalue)
  (`self.SetLifeSpan` AreaDuration))

(fn `UserConstructionScript`)