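; BP_SlowTrailArea is a health effect system actor for a slow-trail area, pairing a mud patch component with a sphere collision.
; On BeginPlay it runs the parent logic, attaches MudPatch to SphereCollision with relative transforms, disables the patch's collision and sets the sphere's object type to Camera.
; The Blueprint itself applies no slow effect; its overlap and tick events are disabled stubs.
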(event `self.ReceiveBeginPlay`
  (bind _mudpatch (`self.MudPatch`))
  (bind _spherecollision (`self.SphereCollision`))
  (`parent.ReceiveBeginPlay`)
  (`SceneComponent.K2_AttachToComponent` _mudpatch _spherecollision "None" "KeepRelative" "KeepRelative" "KeepRelative" true)
  (`PrimitiveComponent.SetCollisionEnabled` _mudpatch "NoCollision")
  (`PrimitiveComponent.SetCollisionObjectType` _spherecollision "ECC_Camera"))

(fn `UserConstructionScript`
  (`parent.UserConstructionScript`))