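; Status effect component that tracks active effects on its owner and whether it can act.
; Effects live in a set of structs with type, remaining time and infinite flag; reapplying keeps the longer time and any infinite flag.
; Applying or removing an effect re-evaluates CanAct, which one specific effect type blocks, and broadcasts OnCanActChanged only when it flips.
; The graphs shown do not count durations down.
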(fn `ApplyStatusEffect`
  (params (Type :type "/Game/Content/Game/HealthSystem/Enums/E_StatusEffect Enum" :default "NewEnumerator0") (Duration :type "Float (double-precision)") (Infifnite :type Boolean))
  (bind _activeeffects (`self.ActiveEffects`))
  (bind (_haseffect _activestatuseffect) (`self.HasStatusEffect` Type))
  (if _haseffect
    (`BlueprintSetLibrary.Set_Remove` _activeeffects _activestatuseffect)
    (bind (_type _remainingtime _binfinite) (break `/Game/Content/Game/HealthSystem/Structs/ST_ActiveStatusEffect` _activestatuseffect))
    (`BlueprintSetLibrary.Set_Add` _activeeffects (make `/Game/Content/Game/HealthSystem/Structs/ST_ActiveStatusEffect` Type (`KismetMathLibrary.FMax` _remainingtime Duration) (or Infifnite _binfinite)))
    (else
      (`BlueprintSetLibrary.Set_Add` _activeeffects (make `/Game/Content/Game/HealthSystem/Structs/ST_ActiveStatusEffect` Type Duration Infifnite))))
  (`self.RecalculateCanAct`))

(fn `HasStatusEffect`
  (params (Type :type "/Game/Content/Game/HealthSystem/Enums/E_StatusEffect Enum" :default "NewEnumerator0"))
  (returns (hasEffect :type Boolean) (ActiveStatusEffect :type "/Game/Content/Game/HealthSystem/Structs/ST_ActiveStatusEffect Structure"))
  (locals (bHasEffect :type Boolean) (ActiveEffect :type "/Game/Content/Game/HealthSystem/Structs/ST_ActiveStatusEffect Structure"))
  (bind _valuepin (`|SetForEach` (`self.ActiveEffects`) :!label _label)
    (:`then`
      (if (`|EnumEquality` (`.Type_2_529D2885434A8B034DEC6DA08AB33541` (break `/Game/Content/Game/HealthSystem/Structs/ST_ActiveStatusEffect` _valuepin)) Type)
        (set `local.bHasEffect` true)
        (set `local.ActiveEffect` _valuepin)
        (goto _label :!via `BreakPin`)))
    (:`CompletedPin`
      (return (`local.bHasEffect`) (`local.ActiveEffect`)))))

(fn `RecalculateCanAct`
  (bind _haseffect (`self.HasStatusEffect` "NewEnumerator2"))
  (bind _returnvalue (not _haseffect))
  (if (!= _returnvalue (`self.bCanAct`))
    (bind _output_get (set `self.bCanAct` _returnvalue))
    (`self.OnCanActChanged` _output_get)))

(fn `RemoveStatusEffect`
  (params (Type :type "/Game/Content/Game/HealthSystem/Enums/E_StatusEffect Enum" :default "NewEnumerator0"))
  (bind (_haseffect _activestatuseffect) (`self.HasStatusEffect` Type))
  (if _haseffect
    (`BlueprintSetLibrary.Set_Remove` (`self.ActiveEffects`) _activestatuseffect)
    (`self.RecalculateCanAct`)))