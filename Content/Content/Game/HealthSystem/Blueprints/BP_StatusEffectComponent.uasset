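; Status effect component that tracks timed or infinite effects on its owner in a map keyed by type.
; Reapplying an effect keeps the later expiry and original magnitude, and Stunned drives CanAct with a change notification.
; Rather than ticking, it sets one timer for the nearest expiry to purge expired effects.
; StartBurning, not called here, starts a looping timer that damages the owner's BP_HealthComponent by the effect's magnitude.
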(event EventBeginPlay)

(event EventTick
  (params (DeltaSeconds :type Float%20%28single-precision%29)))

(fn HasStatusEffect
  (params (Type :type E_StatusEffect%20Enum :default "NewEnumerator0"))
  (bind _activeeffects (Variables|Default|GetActiveEffects))
  (bind (_value _returnvalue) (Utilities|Map|Find _activeeffects Type))
  (return _returnvalue _value))

(fn RecalculateCanAct
  (bind _haseffect (CallFunction|HasStatusEffect "NewEnumerator2"))
  (if (!= (not _haseffect) (Variables|Default|GetbCanAct))
    (bind _output_get (Variables|Default|SetbCanAct (not _haseffect)))
    (Default|CallOnCanActChanged _output_get)))

(fn ApplyStatusEffect
  (params (Type :type E_StatusEffect%20Enum :default "NewEnumerator0") (Duration :type Float%20%28double-precision%29) (Infifnite :type Boolean) (Magnitude :type Float%20%28double-precision%29) (TickInterval :type Float%20%28double-precision%29))
  (bind _activeeffects (Variables|Default|GetActiveEffects))
  (bind (_haseffect _activestatuseffect) (CallFunction|HasStatusEffect Type))
  (if _haseffect
    (Utilities|Map|Remove _activeeffects (.Type (Utilities|Struct|BreakST_ActiveStatusEffect _activestatuseffect)))
    (Utilities|Map|Add _activeeffects Type (Utilities|Struct|MakeST_ActiveStatusEffect Type (Math|Float|Max(Float) (.ExpireAt (Utilities|Struct|BreakST_ActiveStatusEffect _activestatuseffect)) (+ Duration (Utilities|Time|GetGameTimeinSeconds))) (or Infifnite (.bInfinite (Utilities|Struct|BreakST_ActiveStatusEffect _activestatuseffect))) (.Magnitude (Utilities|Struct|BreakST_ActiveStatusEffect _activestatuseffect)) (.TickInterval (Utilities|Struct|BreakST_ActiveStatusEffect _activestatuseffect))))
    (else
      (Utilities|Map|Add _activeeffects Type (Utilities|Struct|MakeST_ActiveStatusEffect Type (+ Duration (Utilities|Time|GetGameTimeinSeconds)) Infifnite Magnitude TickInterval))))
  (CallFunction|RecalculateCanAct)
  (switch Utilities|FlowControl|Switch|SwitchonE_StatusEffect "NewEnumerator0"
    (:NewEnumerator0
      (CallFunction|ScheduleNextStatusExpiration))))

(fn RemoveStatusEffect
  (params (Type :type E_StatusEffect%20Enum :default "NewEnumerator0"))
  (bind (_haseffect _activestatuseffect) (CallFunction|HasStatusEffect Type))
  (if _haseffect
    (Utilities|Map|Remove (Variables|Default|GetActiveEffects) (.type _activestatuseffect))
    (CallFunction|RecalculateCanAct)
    (CallFunction|ScheduleNextStatusExpiration)))

(fn ScheduleNextStatusExpiration
  (Utilities|Time|ClearandInvalidateTimerbyHandle (Variables|Default|GetStatusExpirationTimer))
  (bind _valuepin (Utilities|Map|ForEachLoop(Map) (Variables|Default|GetActiveEffects))
    (:then
      (if (not (.bInfinite (Utilities|Struct|BreakST_ActiveStatusEffect _valuepin)))
        (if (LocalVariables|GetbFoundExpiration)
          (if (< (.ExpireAt (Utilities|Struct|BreakST_ActiveStatusEffect _valuepin)) (LocalVariables|GetNearestExpireAt))
            (LocalVariables|SetNearestExpireAt (.ExpireAt (Utilities|Struct|BreakST_ActiveStatusEffect _valuepin))))
          (else
            (LocalVariables|SetNearestExpireAt (.ExpireAt (Utilities|Struct|BreakST_ActiveStatusEffect _valuepin)))
            (LocalVariables|SetbFoundExpiration true)))))
    (:CompletedPin
      (if (LocalVariables|GetbFoundExpiration)
        (bind _output_get (LocalVariables|SetDelay (|(max(({CBF0877D-4D86-F1F7-4E69-D1AD24D1341D}-now),0.010000)) (Utilities|Time|GetGameTimeinSeconds))))
        (bind _returnvalue (Utilities|Time|SetTimerbyEvent (EventDispatchers|CreateEvent :!event ProcessExpiredStatuses) _output_get))
        (Variables|Default|SetStatusExpirationTimer _returnvalue)))))

(fn ProcessExpiredStatuses
  (bind _activeeffects (Variables|Default|GetActiveEffects))
  (bind _keys (Utilities|Map|Keys _activeeffects))
  (for _array_element _keys
    (if (.ReturnValue (Utilities|Map|Find _activeeffects _array_element))
      (if (and (not (.bInfinite (Utilities|Struct|BreakST_ActiveStatusEffect (.Value (Utilities|Map|Find _activeeffects _array_element))))) (<= (.ExpireAt (Utilities|Struct|BreakST_ActiveStatusEffect (.Value (Utilities|Map|Find _activeeffects _array_element)))) (Utilities|Time|GetGameTimeinSeconds)))
        (Utilities|Map|Remove _activeeffects _array_element))))
  (CallFunction|RecalculateCanAct)
  (CallFunction|ScheduleNextStatusExpiration))

(fn StartBurning
  (bind (_haseffect _activestatuseffect) (CallFunction|HasStatusEffect "NewEnumerator0"))
  (if _haseffect
    (Utilities|Time|SetTimerbyFunctionName 0 "BurningTick" (.TickInterval (Utilities|Struct|BreakST_ActiveStatusEffect _activestatuseffect)) true)))

(fn BurningTick
  (bind _activestatuseffect (CallFunction|HasStatusEffect "NewEnumerator0"))
  (if true
    (Default|HandleDamage (Actor|GetComponentbyClass (Components|GetOwner) "/Game/Content/Game/HealthSystem/Blueprints/BP_HealthComponent.BP_HealthComponent_C") (.Magnitude (Utilities|Struct|BreakST_ActiveStatusEffect _activestatuseffect)) "NewEnumerator0")
    (else
      (Utilities|Time|ClearandInvalidateTimerbyHandle (Variables|Default|GetBurningTimerHandle)))))