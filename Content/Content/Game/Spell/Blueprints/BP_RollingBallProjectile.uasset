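; Rolling mudball spell projectile: a physics sphere that knocks back and damages characters and leaves an area trail.
; Init launches the sphere along the cast direction using speed from the spell definition.
; Overlap skips the caster and prior hits, launches characters along the ball's horizontal velocity with added lift, and damages their health component.
; Tick spawns Niagara mud and short-lived, pulsing status areas at distance intervals.
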(event `self.ReceiveTick`
  (params (DeltaSeconds :type "Float (single-precision)"))
  (`parent.ReceiveTick` DeltaSeconds)
  (`self.TrySpawnTrail`))

(event `self.Sphere.OnComponentBeginOverlap`
  (params (OverlappedComponent :type "PrimitiveComponent Object Reference") (OtherActor :type "Actor Object Reference") (OtherComp :type "PrimitiveComponent Object Reference") (OtherBodyIndex :type Integer) (bFromSweep :type Boolean) (SweepResult :type "HitResult Structure (by ref)"))
  (bind _alreadyhitactors (`self.AlreadyHitActors`))
  (if (== OtherActor (`self.CasterActor`))
    _
    (elif (not (`BlueprintSetLibrary.Set_Contains` _alreadyhitactors OtherActor))
      (bind _returnvalue (`PrimitiveComponent.GetPhysicsLinearVelocity` (`self.Sphere`) "None"))
      (bind _ascharacter (cast `Character` OtherActor))
      (`Character.LaunchCharacter` _ascharacter (`self.NewMacro` (.x _returnvalue) (.y _returnvalue)) true false)
      (`BlueprintSetLibrary.Set_Add` _alreadyhitactors OtherActor)
      (`/Game/Content/Game/HealthEffectSystem/Blueprints/BP_HealthComponent.HandleDamage` (`self.GetComponentByClass` OtherActor "/Game/Content/Game/HealthEffectSystem/Blueprints/BP_HealthComponent.BP_HealthComponent_C") (`/Game/Content/Game/Spell/DataAssets/DA_SpellDefinition.Damage` (`self.SpellDefinition`)) "NewEnumerator2" self))))

(fn `Init`
  (params (Direction :type "Vector Structure") (CasterActor :type "Actor Object Reference") (SpellDefinition :type "/Game/Content/Game/Spell/DataAssets/DA_SpellDefinition Object Reference"))
  (bind _sphere (`self.Sphere`))
  (`parent.Init` Direction CasterActor SpellDefinition)
  (`PrimitiveComponent.SetPhysicsLinearVelocity` _sphere (* (`local.Direction`) (`/Game/Content/Game/Spell/DataAssets/DA_SpellDefinition.ProjectileSpeed` (`local.SpellDefinition`))) false "None")
  (set `self.LastTrailLocation` (`SceneComponent.K2_GetComponentLocation` _sphere)))

(fn `TrySpawnTrail`
  (bind _casteractor (`self.CasterActor`))
  (bind _returnvalue (`SceneComponent.K2_GetComponentLocation` (`self.Sphere`)))
  (if (>= (`KismetMathLibrary.Vector_Distance` _returnvalue (`self.LastTrailLocation`)) (`self.TrailSpacing`))
    (`NiagaraFunctionLibrary.SpawnSystemAtLocation` _casteractor "/Game/Content/Game/VFX/NS_MudballTrail.NS_MudballTrail" _returnvalue)
    (bind _returnvalue_2 (`|SpawnActorFromClass` (`self.TrailAreaClass`) (`KismetMathLibrary.MakeTransform` _returnvalue) "Undefined" "MultiplyWithRoot" null null))
    (`/Game/Content/Game/HealthEffectSystem/Blueprints/BP_AreaEffectBase.InitArea` _returnvalue_2 120.0 2.0 0.2 "NewEnumerator3" 2.0 0.05 0.0 false _casteractor)
    (set `self.LastTrailLocation` _returnvalue)))

(fn `UserConstructionScript`
  (`parent.UserConstructionScript`))