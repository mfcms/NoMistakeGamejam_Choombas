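; Spell behavior for a near-lightning spell that strikes basic enemies around the caster.
; On execute, it loops over all BP_EnemyBasic actors and gates each through a macro containing a caster-distance versus spell-radius comparison, which appears unwired.
; Passing enemies get Niagara strike and pulse effects, the spell's status effect via their status component, and Nature-type damage.
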(fn `ExecuteSpell`
  (params (Spell :type "/Game/Content/Game/Spell/DataAssets/DA_SpellDefinition Object Reference") (Context :type "/Game/Content/Game/Spell/Structs/ST_SpellCastContext Structure"))
  (bind _spell (`local.Spell`))
  (bind _spell_2 (`local.Spell`))
  (bind (_spellsystem _caster _playercontroller) (break `/Game/Content/Game/Spell/Structs/ST_SpellCastContext` (`local.Context`)))
  (`parent.ExecuteSpell` Spell Context)
  (`/Engine/EditorBlueprintResources/StandardMacros.IsValid` _caster
    (:`Is Valid`
      (bind _outactors (`GameplayStatics.GetAllActorsOfClass` _caster "/Game/AI/BP_EnemyBasic.BP_EnemyBasic_C"))
      (for _array_element _outactors
        (if (`self.NewMacro` _array_element _caster _spell)
          (bind _returnvalue (`Actor.K2_GetActorLocation` _array_element))
          (`NiagaraFunctionLibrary.SpawnSystemAtLocation` _caster "/Game/Content/Game/VFX/NS_LightningStrikeSprite.NS_LightningStrikeSprite" (+ _returnvalue (0.0 0.0 225.0)))
          (`NiagaraFunctionLibrary.SpawnSystemAtLocation` _caster "/Game/Content/Game/VFX/NS_LightningPulse.NS_LightningPulse" _returnvalue)
          (`/Game/Content/Game/HealthEffectSystem/Blueprints/BP_StatusEffectComponent.ApplyStatusEffect` (`Actor.GetComponentByClass` _array_element "/Game/Content/Game/HealthEffectSystem/Blueprints/BP_StatusEffectComponent.BP_StatusEffectComponent_C") (`/Game/Content/Game/Spell/DataAssets/DA_SpellDefinition.StatusEffect` _spell_2) (`/Game/Content/Game/Spell/DataAssets/DA_SpellDefinition.StatusDuration` _spell_2) (`/Game/Content/Game/Spell/DataAssets/DA_SpellDefinition.StatusInfinite` _spell_2) (`/Game/Content/Game/Spell/DataAssets/DA_SpellDefinition.StatusMagnitude` _spell_2) (`/Game/Content/Game/Spell/DataAssets/DA_SpellDefinition.StatusTickInterval` _spell_2))
          (`GameplayStatics.ApplyDamage` _array_element (`/Game/Content/Game/Spell/DataAssets/DA_SpellDefinition.Damage` _spell) _playercontroller _caster "/Game/Content/Game/HealthEffectSystem/Blueprints/BP_DT_Nature.BP_DT_Nature_C"))))))