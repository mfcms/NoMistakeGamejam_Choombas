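; Fireball spell projectile that explodes on hit, dealing radial fire damage and applying a status effect to nearby pawns.
; Init takes speed, damage and radius from the spell definition, launches along local X, enables collision and starts a looping timer spawning Niagara trail puffs.
; Hits before initialization or on the caster are ignored; Explode spawns impact VFX, spares the caster, passes status settings to each BP_StatusEffectComponent, then destroys the projectile.
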(event `SpawnFireTrailPuff`
  (`NiagaraFunctionLibrary.SpawnSystemAtLocation` "/Game/Content/Game/VFX/NS_FireballTrail.NS_FireballTrail" (`self.K2_GetActorLocation`)))

(event `self.SphereCollision.OnComponentHit`
  (params (HitComponent :type "PrimitiveComponent Object Reference") (OtherActor :type "Actor Object Reference") (OtherComp :type "PrimitiveComponent Object Reference") (NormalImpulse :type "Vector Structure") (Hit :type "HitResult Structure (by ref)"))
  (if (not (or (== OtherActor (`self.Caster`)) (not (`self.bInitialized`))))
    (`KismetSystemLibrary.PrintString` (`KismetSystemLibrary.GetObjectName` OtherActor))
    (`self.Explode`)))

(fn `Explode`
  (bind _returnvalue (`self.K2_GetActorLocation`))
  (bind _spelldefinition (`self.SpellDefinition`))
  (bind _caster (`self.Caster`))
  (bind _explosionradius (`self.ExplosionRadius`))
  (bind _array (`|MakeArray` _caster))
  (`NiagaraFunctionLibrary.SpawnSystemAtLocation` "/Game/Content/Game/VFX/NS_FireballImpact.NS_FireballImpact" _returnvalue)
  (`GameplayStatics.ApplyRadialDamage` (`self.Damage`) _returnvalue _explosionradius "/Game/Content/Game/HealthEffectSystem/Blueprints/BP_DT_Fire.BP_DT_Fire_C" _array self (`self.GetInstigatorController` _caster) true)
  (bind _outactors (`KismetSystemLibrary.SphereOverlapActors` _returnvalue _explosionradius (`|MakeArray` "ObjectTypeQuery3" :!type "EObjectTypeQuery Enum") null _array))
  (for _array_element _outactors
    (bind _returnvalue_2 (`self.GetComponentByClass` _array_element "/Game/Content/Game/HealthEffectSystem/Blueprints/BP_StatusEffectComponent.BP_StatusEffectComponent_C"))
    (if (`KismetSystemLibrary.IsValid` _returnvalue_2)
      (`/Game/Content/Game/HealthEffectSystem/Blueprints/BP_StatusEffectComponent.ApplyStatusEffect` _returnvalue_2 (`/Game/Content/Game/Spell/DataAssets/DA_SpellDefinition.StatusEffect` _spelldefinition) (`/Game/Content/Game/Spell/DataAssets/DA_SpellDefinition.Duration` _spelldefinition) (`/Game/Content/Game/Spell/DataAssets/DA_SpellDefinition.StatusInfinite` _spelldefinition) (`/Game/Content/Game/Spell/DataAssets/DA_SpellDefinition.StatusMagnitude` _spelldefinition) (`/Game/Content/Game/Spell/DataAssets/DA_SpellDefinition.StatusTickInterval` _spelldefinition))))
  (`self.K2_DestroyActor`))

(fn `Init`
  (params (Direction :type "Vector Structure") (CasterActor :type "Actor Object Reference") (SpellDefinition :type "/Game/Content/Game/Spell/DataAssets/DA_SpellDefinition Object Reference"))
  (`parent.Init` Direction CasterActor SpellDefinition)
  (`self.InitFireball` Direction (`/Game/Content/Game/Spell/DataAssets/DA_SpellDefinition.ProjectileSpeed` SpellDefinition) (`/Game/Content/Game/Spell/DataAssets/DA_SpellDefinition.Damage` SpellDefinition) (`/Game/Content/Game/Spell/DataAssets/DA_SpellDefinition.Radius` SpellDefinition) CasterActor))

(fn `InitFireball`
  (params (Direction :type "Vector Structure") (Speed :type "Float (double-precision)") (DamageValue :type "Float (double-precision)") (RadiusValue :type "Float (double-precision)") (CasterActor :type "Actor Object Reference"))
  (set `self.Damage` DamageValue)
  (set `self.ExplosionRadius` RadiusValue)
  (bind _output_get (set `self.Caster` CasterActor))
  (`ProjectileMovementComponent.SetVelocityInLocalSpace` (`self.ProjectileMovement`) (`KismetMathLibrary.MakeVector` Speed))
  (`PrimitiveComponent.IgnoreActorWhenMoving` (`self.SphereCollision`) _output_get true)
  (set `self.bInitialized` true)
  (`PrimitiveComponent.SetCollisionEnabled` (`self.SphereCollision`) "QueryOnly")
  (`KismetSystemLibrary.K2_SetTimer` null "SpawnFireTrailPuff" 0.065 true))

(fn `UserConstructionScript`)