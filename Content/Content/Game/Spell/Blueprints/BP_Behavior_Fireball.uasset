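; Fireball spell behavior that launches a fireball projectile from the caster toward the cursor hit point, doing nothing without a hit.
; The spell system spawns BP_FireballProjectile, which is then initialized with direction, the spell's speed, damage and radius, and the caster.
; A helper flattens the caster-to-cursor vector to horizontal and builds the spawn transform slightly ahead of and above the caster, facing that direction.
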(fn `ExecuteSpell`
  (params (Spell :type "/Game/Content/Game/Spell/DataAssets/DA_SpellDefinition Object Reference") (Context :type "/Game/Content/Game/Spell/Structs/ST_SpellCastContext Structure"))
  (bind (_spellsystem _caster _playercontroller _cursorlocation _cursornormal _hascursorhit) (break `/Game/Content/Game/Spell/Structs/ST_SpellCastContext` Context))
  (bind (_returnvalue _direction) (`self.GetSpawnLocation` _cursorlocation (`Actor.K2_GetActorLocation` _caster)))
  (if _hascursorhit
    (bind _spawnedactor (`/Game/Content/Game/Spell/Blueprints/BP_SpellSystemComponent.SpawnSpellActor` _spellsystem "/Game/Content/Game/Spell/Blueprints/BP_FireballProjectile.BP_FireballProjectile_C" _returnvalue))
    (bind _asbp_fireball_projectile (cast `/Game/Content/Game/Spell/Blueprints/BP_FireballProjectile` _spawnedactor))
    (`/Game/Content/Game/Spell/Blueprints/BP_FireballProjectile.InitFireball` _asbp_fireball_projectile _direction (`/Game/Content/Game/Spell/DataAssets/DA_SpellDefinition.ProjectileSpeed` Spell) (`/Game/Content/Game/Spell/DataAssets/DA_SpellDefinition.Damage` Spell) (`/Game/Content/Game/Spell/DataAssets/DA_SpellDefinition.Radius` Spell) _caster)
    (else
      (return))))