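; Tornado spell projectile that knocks back what it overlaps, dealing air damage from its spell definition.
; Init sets velocity, force and caster, then enables query-only sphere collision.
; Each new overlapped actor except the caster goes to PushActor: Characters receive the status effect and are launched, while physics-simulating roots get an impulse.
; Both cases take damage and stop the projectile's movement without destroying it.
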(event `self.SphereCollision.OnComponentBeginOverlap`
  (params (OverlappedComponent :type "PrimitiveComponent Object Reference") (OtherActor :type "Actor Object Reference") (OtherComp :type "PrimitiveComponent Object Reference") (OtherBodyIndex :type Integer) (bFromSweep :type Boolean) (SweepResult :type "HitResult Structure (by ref)"))
  (bind _alreadyhitactors (`self.AlreadyHitActors`))
  (bind _other_actor (`self.Other Actor`))
  (set `self.Other Actor` OtherActor)
  (if (`BlueprintSetLibrary.Set_Contains` _alreadyhitactors (`self.Other Actor`))
    _
    (elif (not (or (== (`self.Other Actor`) (`self.Caster`)) (not (`self.bInitialized`))))
      (`BlueprintSetLibrary.Set_Add` _alreadyhitactors _other_actor)
      (`KismetSystemLibrary.PrintString` (`KismetSystemLibrary.GetObjectName` _other_actor))
      (`self.PushActor` _other_actor))))

(fn `Init`
  (params (Direction :type "Vector Structure") (CasterActor :type "Actor Object Reference") (SpellDefinition :type "/Game/Content/Game/Spell/DataAssets/DA_SpellDefinition Object Reference"))
  (`parent.Init` Direction CasterActor SpellDefinition)
  (`self.InitTornado` Direction (`/Game/Content/Game/Spell/DataAssets/DA_SpellDefinition.ProjectileSpeed` SpellDefinition) (`/Game/Content/Game/Spell/DataAssets/DA_SpellDefinition.Damage` SpellDefinition) CasterActor (`/Game/Content/Game/Spell/DataAssets/DA_SpellDefinition.Force` SpellDefinition)))

(fn `InitTornado`
  (params (Direction :type "Vector Structure") (Speed :type "Float (double-precision)") (DamageValue :type "Float (double-precision)") (CasterActor :type "Actor Object Reference") (Force :type "Float (double-precision)"))
  (`KismetSystemLibrary.PrintString` (`KismetStringLibrary.Conv_DoubleToString` Speed))
  (set `self.Damage` DamageValue)
  (set `self.Force` Force)
  (bind _output_get (set `self.Caster` CasterActor))
  (`ProjectileMovementComponent.SetVelocityInLocalSpace` (`self.ProjectileMovement`) (`KismetMathLibrary.MakeVector` Speed))
  (`PrimitiveComponent.IgnoreActorWhenMoving` (`self.SphereCollision`) _output_get true)
  (set `self.bInitialized` true)
  (`PrimitiveComponent.SetCollisionEnabled` (`self.SphereCollision`) "QueryOnly"))

(fn `PushActor`
  (params (ActorToPush :type "Actor Object Reference"))
  (bind _launchvector (`self.GetLaunchVector`))
  (bind _spelldefinition (`self.SpellDefinition`))
  (if (`KismetSystemLibrary.IsValid` ActorToPush)
    (bind _ascharacter (cast `Character` ActorToPush)
      (:`then`
        (`/Game/Content/Game/HealthEffectSystem/Blueprints/BP_StatusEffectComponent.ApplyStatusEffect` (`self.GetComponentByClass` ActorToPush "/Game/Content/Game/HealthEffectSystem/Blueprints/BP_StatusEffectComponent.BP_StatusEffectComponent_C") (`/Game/Content/Game/Spell/DataAssets/DA_SpellDefinition.StatusEffect` _spelldefinition) (`/Game/Content/Game/Spell/DataAssets/DA_SpellDefinition.StatusDuration` _spelldefinition) (`/Game/Content/Game/Spell/DataAssets/DA_SpellDefinition.StatusInfinite` _spelldefinition) (`/Game/Content/Game/Spell/DataAssets/DA_SpellDefinition.StatusMagnitude` _spelldefinition) (`/Game/Content/Game/Spell/DataAssets/DA_SpellDefinition.StatusTickInterval` _spelldefinition))
        (`Character.LaunchCharacter` _ascharacter _launchvector true true)
        (`GameplayStatics.ApplyDamage` ActorToPush (`/Game/Content/Game/Spell/DataAssets/DA_SpellDefinition.Damage` _spelldefinition) null (`self.Caster`) "/Game/Content/Game/HealthEffectSystem/Blueprints/BP_DT_Air.BP_DT_Air_C" :!label _label)
        (`MovementComponent.StopMovementImmediately` (`self.ProjectileMovement`)))
      (:`CastFailed`
        (bind _asprimitive_component (cast `PrimitiveComponent` (`Actor.RootComponent` ActorToPush)))
        (if (`SceneComponent.IsSimulatingPhysics` _asprimitive_component "None")
          (`PrimitiveComponent.AddImpulse` _asprimitive_component _launchvector "None" true)
          (goto _label))))))

(fn `UserConstructionScript`)