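; Spell-casting component that builds spells from staged button inputs: two elements and a paradigm.
; Each input advances the stage, and button-to-option mapping rotates after each round unless disabled.
; Completed combinations are matched against KnownSpells, then a constructed behavior object executes with caster and cursor-hit context.
; Ruined or unknown spells backfire by first element: Fire status effect, Water status and movement stop, Nature silence, or Air launch with landing damage.
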(event `self.ReceiveBeginPlay`)

(fn `EndBeat`
  (bind _currentstageindex (`self.CurrentStageIndex`))
  (if (`self.bInputReceived`)
    _
    (else
      _))
  (if (== _currentstageindex (- (`KismetArrayLibrary.Array_Length` (`self.Stages`)) 1))
    (set `self.CurrentStageIndex` 0)
    (`self.EndRound`)
    (else
      (set `self.CurrentStageIndex` (+ _currentstageindex 1))
      (`self.StartBeat`))))

(fn `EndRound`
  (locals (bNoSwapHack :type Boolean :default true))
  (if (not (`local.bNoSwapHack`))
    (set `self.ButtonOffset` (mod (+ (`self.ButtonOffset`) 1) 4)))
  (`self.ResolveSpell`)
  (`self.StartRound`)
  (`self.StartBeat`))

(fn `ExecuteResolvedSpell`
  (params (Spell :type "/Game/Content/Game/Spell/DataAssets/DA_SpellDefinition Object Reference"))
  (bind _returnvalue (`GameplayStatics.GetPlayerController` 0))
  (bind (_bblockinghit _binitialoverlap _time _distance _location _impactpoint _normal _impactnormal) (`GameplayStatics.BreakHitResult` (`PlayerController.GetHitResultUnderCursorByChannel` _returnvalue "TraceTypeQuery1" false)))
  (bind _returnvalue_2 (`|GenericCreateObject` self (`/Game/Content/Game/Spell/DataAssets/DA_SpellDefinition.BehaviorClass` Spell)))
  (`/Game/Content/Game/Spell/Blueprints/BP_SpellBehaviorB.ExecuteSpell` _returnvalue_2 Spell (make `/Game/Content/Game/Spell/Structs/ST_SpellCastContext` self (`self.GetOwner`) _returnvalue _impactpoint _impactnormal _bblockinghit)))

(fn `GetOptionForButton`
  (params (InputIndex :type Integer))
  (returns (Option :type "/Game/Content/Game/Spell/Structs/ST_SpellOption Structure"))
  (return (`|GetArrayItem` (`.Options_6_6C4A02074D159EEAD69EBBB3C4FDC8DD` (break `/Game/Content/Game/Spell/Structs/ST_SpellStage` (`|GetArrayItem` (`self.Stages`) (`self.CurrentStageIndex`)))) (mod (+ InputIndex (`self.ButtonOffset`)) 4))))

(fn `HandleAirMiscastLanding`
  (bind _returnvalue (`self.GetOwner`))
  (if (`self.bAirMiscastPending`)
    (set `self.bAirMiscastPending` false)
    (`NiagaraFunctionLibrary.SpawnSystemAtLocation` _returnvalue "/Game/Content/Game/VFX/NS_AirLanding.NS_AirLanding" (`Actor.K2_GetActorLocation` _returnvalue))
    (`GameplayStatics.ApplyDamage` _returnvalue 20.0 null _returnvalue "/Game/Content/Game/HealthEffectSystem/Blueprints/BP_DT_Air.BP_DT_Air_C")))

(fn `ResolveMiscast`
  (params (Element :type "/Game/Content/Game/Spell/Enums/E_SpellToken Enum" :default "NewEnumerator8"))
  (bind _returnvalue (`self.GetOwner`))
  (bind _returnvalue_2 (`Actor.GetComponentByClass` _returnvalue "/Game/Content/Game/HealthEffectSystem/Blueprints/BP_StatusEffectComponent.BP_StatusEffectComponent_C"))
  (bind _returnvalue_3 (`Actor.K2_GetRootComponent` _returnvalue))
  (switch `/Game/Content/Game/Spell/Enums/E_SpellToken` Element
    (:`NewEnumerator0`
      (`/Game/Content/Game/HealthEffectSystem/Blueprints/BP_StatusEffectComponent.ApplyStatusEffect` _returnvalue_2 "NewEnumerator0" 3.0 false 5.0 1.0))
    (:`NewEnumerator1`
      (`/Game/Content/Game/HealthEffectSystem/Blueprints/BP_StatusEffectComponent.ApplyStatusEffect` _returnvalue_2 "NewEnumerator2" 2.0 false 0.0 0.0)
      (`Controller.StopMovement` (`GameplayStatics.GetPlayerController` _returnvalue)))
    (:`NewEnumerator2`
      (set `self.SilencedUntil` (+ (`KismetSystemLibrary.GetGameTimeInSeconds` _returnvalue) 5.0))
      (`NiagaraFunctionLibrary.SpawnSystemAttached` "/Game/Content/Game/VFX/NS_Silenced.NS_Silenced" _returnvalue_3 "None" (0.0 0.0 110.0) (struct) "KeepRelativeOffset" true true "None" false))
    (:`NewEnumerator3`
      (set `self.bAirMiscastPending` true)
      (`NiagaraFunctionLibrary.SpawnSystemAttached` "/Game/Content/Game/VFX/NS_AirLift.NS_AirLift" _returnvalue_3 "None" (0.0 0.0 60.0) (struct) "KeepRelativeOffset" true true "None" false)
      (`Character.LaunchCharacter` (`GameplayStatics.GetPlayerCharacter` _returnvalue) (`KismetMathLibrary.MakeVector` 0.0 0.0 900.0) false true))))

(fn `ResolveSpell`
  (locals (bSpellFound :type Boolean) (ResolvedSpell :type "/Game/Content/Game/Spell/DataAssets/DA_SpellDefinition Object Reference") (DefaultMiscastSpell :type "/Game/Content/Game/Spell/DataAssets/DA_SpellDefinition Object Reference" :default "/Game/Content/Game/Spell/DataAssets/DA_SpellDefinition.DA_SpellDefinition_C'/Game/Content/Game/Spell/DataAssets/DA_Fireball.DA_Fireball'"))
  (bind _firstspokenelement (`self.FirstSpokenElement`))
  (bind _currentselections (`self.CurrentSelections`))
  (bind _currentselections_2 (`self.CurrentSelections`))
  (if (`self.bSpellRuined`)
    (`KismetSystemLibrary.PrintString` "RUINED SPELL")
    (`self.ResolveMiscast` _firstspokenelement)
    (else
      (`KismetSystemLibrary.PrintString` (`KismetTextLibrary.Conv_TextToString` (`|FormatText` "{0} / {1} / {2}" (`|GetEnumeratorNameAsString` (`|GetArrayItem` _currentselections_2)) (`|GetEnumeratorNameAsString` (`|GetArrayItem` _currentselections_2 1)) (`|GetEnumeratorNameAsString` (`|GetArrayItem` _currentselections_2 2)))))
      (set `local.bSpellFound` false)
      (set `local.ResolvedSpell` null)
      (for _array_element (`self.KnownSpells`)
        (if (and (`|EnumEquality` (`/Game/Content/Game/Spell/DataAssets/DA_SpellDefinition.Element1` _array_element) (`|GetArrayItem` _currentselections)) (`|EnumEquality` (`/Game/Content/Game/Spell/DataAssets/DA_SpellDefinition.Element2` _array_element) (`|GetArrayItem` _currentselections 1)) (`|EnumEquality` (`/Game/Content/Game/Spell/DataAssets/DA_SpellDefinition.Paradigm` _array_element) (`|GetArrayItem` _currentselections 2)))
          (set `local.bSpellFound` true)
          (set `local.ResolvedSpell` _array_element)
          (break)))
      (if (`local.bSpellFound`)
        (`self.ExecuteResolvedSpell` (`local.ResolvedSpell`))
        (else
          (`self.ResolveMiscast` _firstspokenelement))))))

(fn `SetCurrentStageValue`
  (params (Value :type "/Game/Content/Game/Spell/Enums/E_SpellToken Enum" :default "NewEnumerator8"))
  (`KismetArrayLibrary.Array_Set` (`self.CurrentSelections`) (`self.CurrentStageIndex`) Value))

(fn `SpawnSpellActor`
  (params (ActorClass :type "Actor Class Reference") (Transform :type "Transform Structure"))
  (returns (SpawnedActor :type "Actor Object Reference"))
  (bind _returnvalue (`|SpawnActorFromClass` ActorClass Transform "AlwaysSpawn" "MultiplyWithRoot" null null))
  (return _returnvalue))

(fn `StartBeat`
  (set `self.bInputReceived` false)
  (`KismetSystemLibrary.PrintString` (`|GetEnumeratorNameAsString` (`.StageType_2_EF63930C402712452D919CB9B69C8F96` (break `/Game/Content/Game/Spell/Structs/ST_SpellStage` (`|GetArrayItem` (`self.Stages`) (`self.CurrentStageIndex`)))))))

(fn `StartRound`
  (bind _currentselections (`self.CurrentSelections`))
  (`KismetArrayLibrary.Array_Clear` _currentselections)
  (`KismetArrayLibrary.Array_Add` _currentselections "NewEnumerator8")
  (`KismetArrayLibrary.Array_Add` _currentselections "NewEnumerator8")
  (`KismetArrayLibrary.Array_Add` _currentselections "NewEnumerator8")
  (set `self.CurrentStageIndex` 0)
  (set `self.bSpellRuined` false)
  (set `self.bInputReceived` false)
  (set `self.FirstSpokenElement` "NewEnumerator8"))

(fn `TryInputSpellOption`
  (params (InputIndex :type Integer))
  (bind _returnvalue (`self.GetOwner`))
  (bind _haseffect (`/Game/Content/Game/HealthEffectSystem/Blueprints/BP_StatusEffectComponent.HasStatusEffect` (`Actor.GetComponentByClass` _returnvalue "/Game/Content/Game/HealthEffectSystem/Blueprints/BP_StatusEffectComponent.BP_StatusEffectComponent_C") "NewEnumerator2"))
  (if _haseffect
    _
    (elif (< (`KismetSystemLibrary.GetGameTimeInSeconds` _returnvalue) (`self.SilencedUntil`))
      _
      (elif (`self.bInputReceived`)
        (set `self.bSpellRuined` true)
        (`KismetSystemLibrary.PrintString` "DOUBLE INPUT")
        (else
          (bind _option (`self.GetOptionForButton` InputIndex))
          (if (and (== (`self.FirstSpokenElement`) 0) (< (`self.CurrentStageIndex`) 2))
            (bind (_id _displayname) (break `/Game/Content/Game/Spell/Structs/ST_SpellOption` _option))
            (set `self.FirstSpokenElement` _id))
          (`self.SetCurrentStageValue` _id)
          (set `self.bInputReceived` true)
          (`KismetSystemLibrary.PrintText` _displayname)
          (`self.EndBeat`))))))