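; Zombie enemy AI that chases the player and attacks at close range, built on inherited movement and attack hooks.
; Each AI update moves toward the player pawn when beyond the attack radius, otherwise tries to attack; reaching the player also triggers an attempt.
; An attack plays a random attack animation lasting the cooldown and spawns an effect oriented along the flattened player direction with a 180-degree rotation offset.
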(event `self.OnUpdateAI`
  (if (> (`self.DistanceToPlayer`) (`self.AttackRadius`))
    (`self.OnMoveTo` (0.0 0.0 0.0) (`GameplayStatics.GetPlayerPawn` 0) (`self.WalkToRadius`))
    (else
      (`self.TryAttack` :!label _label))))

(event `self.OnMoveToSuccess`
  (goto _label))

(event `self.OnAttack`
  (`self.Attack`))

(event `self.ReceiveBeginPlay`
  (`parent.ReceiveBeginPlay`))

(fn `Attack`
  (bind (_returnvalue_x _returnvalue_y _returnvalue_z) (`KismetMathLibrary.BreakVector` (`self.K2_GetActorLocation`)))
  (bind (_returnvalue_x_2 _returnvalue_y_2) (`KismetMathLibrary.BreakVector` (`self.K2_GetActorLocation` (`GameplayStatics.GetPlayerPawn` 0))))
  (bind _returnvalue (`KismetMathLibrary.MakeVector` _returnvalue_x _returnvalue_y _returnvalue_z))
  (`self.PlayRandomAnimationFor` "Attack" false (`self.AttackCooldown`))
  (`NiagaraFunctionLibrary.SpawnSystemAtLocation` null _returnvalue (`KismetMathLibrary.ComposeRotators` (`KismetMathLibrary.FindLookAtRotation` _returnvalue (`KismetMathLibrary.MakeVector` _returnvalue_x_2 _returnvalue_y_2 _returnvalue_z)) (struct :`Roll` 180.0)) (1.0 1.0 1.0) true true "AutoRelease"))

(fn `UserConstructionScript`
  (`parent.UserConstructionScript`))