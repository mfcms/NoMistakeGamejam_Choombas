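; Ranged enemy AI that fires arrow projectiles at the player, built on a parent class that supplies movement and attack events.
; Each AI update tries to attack when the player's distance is inside the attack range, otherwise it moves to mid-range along the line from player to enemy.
; Unless on cooldown, an attack plays a random animation timed to the cooldown, then spawns an arrow facing the player and initialised with them as target.
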(event `OnMoveInAttackRange`
  (bind (_attackrange_min _attackrange_max) (break `FloatInterval` (`self.AttackRange`)))
  (bind _returnvalue (`self.K2_GetActorLocation` (`GameplayStatics.GetPlayerPawn` 0)))
  (`self.OnMoveTo` (+ (* (`KismetMathLibrary.Normal` (- (`self.K2_GetActorLocation`) _returnvalue)) (/ (+ _attackrange_min _attackrange_max) 2.0)) _returnvalue)))

(event `self.OnUpdateAI`
  (bind (_attackrange_min _attackrange_max) (break `FloatInterval` (`self.AttackRange`)))
  (if (`KismetMathLibrary.InRange_FloatFloat` (`self.DistanceToPlayer`) _attackrange_min _attackrange_max)
    (`self.TryAttack`)
    (else
      (`self.OnMoveInAttackRange`))))

(event `self.OnAttack`
  (`self.Attack`))

(event `self.ReceiveBeginPlay`
  (`parent.ReceiveBeginPlay`))

(fn `Attack`
  (bind _returnvalue (`self.GetTransform`))
  (if (not (`self.AttackOnCooldown`))
    (`self.PlayRandomAnimationFor` "Attack" false (`self.AttackCooldown`))
    (bind _returnvalue_2 (`|SpawnActorFromClass` "/Game/AI/BP/BP_AIProjectileArrow.BP_AIProjectileArrow_C" _returnvalue "Undefined" "MultiplyWithRoot" null 400.0 null))
    (`self.K2_SetActorRotation` _returnvalue_2 (`KismetMathLibrary.FindLookAtRotation` (.location _returnvalue) (`self.K2_GetActorLocation` (`GameplayStatics.GetPlayerPawn` 0))) false)
    (`/Game/AI/BP/BP_AIProjectile.InitProjectile` _returnvalue_2 (`GameplayStatics.GetPlayerPawn` 0) (0.0 0.0 0.0))))

(fn `UserConstructionScript`
  (`parent.UserConstructionScript`))