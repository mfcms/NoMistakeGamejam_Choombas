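; Base enemy with shared movement, attack, damage and death logic, leaving AI updates, attacks and move results as empty event hooks.
; A looping timer runs AI updates while StatusComponent allows acting, which also gates movement and cooldown-limited attacks.
; Typed damage feeds HealthComponent, Tick toggles status VFX and tracks player distance, and player spell hits kill outright.
; Random per-type animations play directly on the mesh, and death delays destruction until the animation ends.
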(event `OnMoveTo`
  (params (Destination :type "Vector Structure") (Target :type "Actor Object Reference") (AcceptanceRadius :type "Float (double-precision)" :default 50.0))
  (if (`/Game/Content/Game/HealthEffectSystem/Blueprints/BP_StatusEffectComponent.bCanAct` (`self.StatusComponent`))
    (`|AIMoveTo` self Destination Target AcceptanceRadius
      (:`then`
        (`self.PlayRandomAnimationFor` "Walk" true))
      (:`OnSuccess`
        (`self.OnMoveToSuccess`))
      (:`OnFail`
        (`self.OnMoveToFailure` :!label _label)))
    (else
      (goto _label))))

(event `OnMoveToSuccess`)

(event `OnMoveToFailure`)

(event `OnAttack`)

(event `OnAttackCooldownEnd`
  (set `self.AttackOnCooldown` false))

(event `OnUpdateAI`)

(event `UpdateAIIfAllowed`
  (if (`/Game/Content/Game/HealthEffectSystem/Blueprints/BP_StatusEffectComponent.bCanAct` (`self.StatusComponent`))
    (`self.OnUpdateAI`)))

(event `self.ReceiveBeginPlay`
  (bind _capsulecomponent (`self.CapsuleComponent`))
  (bind _statuscomponent (`self.StatusComponent`))
  (`SceneComponent.K2_AttachToComponent` (`self.VFX_Burning`) _capsulecomponent "None" "KeepRelative" "KeepRelative" "KeepRelative" true)
  (`SceneComponent.K2_AttachToComponent` (`self.VFX_Stunned`) _capsulecomponent "None" "KeepRelative" "KeepRelative" "KeepRelative" true)
  (`SceneComponent.K2_AttachToComponent` (`self.VFX_Slowed`) _capsulecomponent "None" "KeepRelative" "KeepRelative" "KeepRelative" true)
  (add `/Game/Content/Game/HealthEffectSystem/Blueprints/BP_HealthComponent.OnDeath` (`self.HealthComponent`) (`|CreateDelegate` :!event `Die`))
  (bind _returnvalue (`KismetSystemLibrary.K2_SetTimerDelegate` (delegate `UpdateAIIfAllowed`) (`self._BehUpdateTimer`) true))
  (set `self.UpdateAIHandle` _returnvalue)
  (`self.PlayRandomAnimationFor` "Walk" true)
  (bind _speed (`/Game/Content/Game/HealthEffectSystem/Blueprints/BP_StatusEffectComponent.GetConfiguredWalkSpeed` _statuscomponent (`self.MaxSpeed`)))
  (`/Game/Content/Game/HealthEffectSystem/Blueprints/BP_StatusEffectComponent.SetDesiredWalkSpeed` _statuscomponent _speed))

(event `self.ReceiveTick`
  (params (DeltaSeconds :type "Float (single-precision)"))
  (bind _statuscomponent (`self.StatusComponent`))
  (bind _haseffect (`/Game/Content/Game/HealthEffectSystem/Blueprints/BP_StatusEffectComponent.HasStatusEffect` _statuscomponent "NewEnumerator0"))
  (`ActorComponent.SetActive` (`self.VFX_Burning`) _haseffect false)
  (bind _haseffect_2 (`/Game/Content/Game/HealthEffectSystem/Blueprints/BP_StatusEffectComponent.HasStatusEffect` _statuscomponent "NewEnumerator2"))
  (`ActorComponent.SetActive` (`self.VFX_Stunned`) _haseffect_2 false)
  (bind _haseffect_3 (`/Game/Content/Game/HealthEffectSystem/Blueprints/BP_StatusEffectComponent.HasStatusEffect` _statuscomponent "NewEnumerator3"))
  (`ActorComponent.SetActive` (`self.VFX_Slowed`) _haseffect_3 false)
  (set `self.DistanceToPlayer` (`KismetMathLibrary.Distance2D` (`KismetMathLibrary.Conv_VectorToVector2D` (`self.K2_GetActorLocation`)) (`KismetMathLibrary.Conv_VectorToVector2D` (`self.K2_GetActorLocation` (`GameplayStatics.GetPlayerPawn` 0))))))

(event `self.ReceiveAnyDamage`
  (params (Damage :type "Float (single-precision)") (DamageType :type "DamageType Object Reference") (InstigatedBy :type "Controller Object Reference") (DamageCauser :type "Actor Object Reference"))
  (bind _asbp_damage_type_base (cast `/Game/Content/Game/HealthEffectSystem/Blueprints/BP_DamageTypeBase` DamageType))
  (`/Game/Content/Game/HealthEffectSystem/Blueprints/BP_HealthComponent.HandleDamage` (`self.HealthComponent`) Damage (`/Game/Content/Game/HealthEffectSystem/Blueprints/BP_DamageTypeBase.DamageType` _asbp_damage_type_base) DamageCauser))

(event `self.StatusComponent.OnCanActChanged`
  (params (CanAct :type Boolean))
  (bind _returnvalue (`self.GetController`))
  (if (not CanAct)
    (`self.StopAnimation`)
    (if (`KismetSystemLibrary.IsValid` _returnvalue)
      (`Controller.StopMovement` _returnvalue))))

(event `OnDelayedDestroy`
  (`KismetSystemLibrary.Delay` (+ (`AnimationAsset.GetPlayLength` (`self.LastStartedAnimation`)) 1.0))
  (`self.K2_DestroyActor`))

(event `self.ReceiveHit`
  (params (MyComp :type "PrimitiveComponent Object Reference") (Other :type "Actor Object Reference") (OtherComp :type "PrimitiveComponent Object Reference") (bSelfMoved :type Boolean) (HitLocation :type "Vector Structure") (HitNormal :type "Vector Structure") (NormalImpulse :type "Vector Structure") (Hit :type "HitResult Structure (by ref)"))
  (if (`self.ActorHasTag` Other "PlayerSpell")
    (`self.Die`)))

(fn `Die`
  (bind _charactermovement (`self.CharacterMovement`))
  (`KismetSystemLibrary.K2_ClearAndInvalidateTimerHandle` (`self.UpdateAIHandle`))
  (`NavMovementInterface.StopActiveMovement` _charactermovement)
  (`CharacterMovementComponent.DisableMovement` _charactermovement)
  (`PrimitiveComponent.SetCollisionEnabled` (`self.CapsuleComponent`) "NoCollision")
  (`Controller.UnPossess` (`self.GetController`))
  (`self.OnDie`)
  (`self.PlayRandomAnimationFor` "Death")
  (`self.OnDelayedDestroy`))

(fn `GetRandomAnimationFor`
  (params (Type :type String))
  (returns (Animation :type "AnimationAsset Object Reference"))
  (bind (_value _returnvalue) (`BlueprintMapLibrary.Map_Find` (`self.Animations`) Type))
  (bind _animations (break `/Game/AI/STR_AnimationsList` _value))
  (if (and _returnvalue (> (`KismetArrayLibrary.Array_Length` _animations) 0))
    (return (`KismetArrayLibrary.Array_Random` _animations))
    (else
      (return "/Game/Characters/Enemies/MobAnims/Rig_Medium_GeneralT-Pose.Rig_Medium_GeneralT-Pose"))))

(fn `PlayRandomAnimationFor`
  (params (Type :type String) (Looping :type Boolean) (OverrideDuration :type "Float (double-precision)" :default -1.0))
  (bind _overrideduration (`local.OverrideDuration`))
  (bind _mesh (`self.Mesh`))
  (if (or (`KismetStringLibrary.NotEqual_StrStr` (`self.PlayingAnimation`) Type) (not Looping))
    (bind _animation (`self.GetRandomAnimationFor` Type))
    (`SkeletalMeshComponent.PlayAnimation` (`self.Mesh`) _animation Looping)
    (set `self.LastStartedAnimation` _animation)
    (if (> _overrideduration 0.0)
      (`SkeletalMeshComponent.SetPlayRate` _mesh (/ (`AnimationAsset.GetPlayLength` _animation) _overrideduration))
      (else
        (`SkeletalMeshComponent.SetPlayRate` _mesh 1.0)))
    (set `self.PlayingAnimation` Type)))

(fn `StartAttackCooldown`
  (`KismetSystemLibrary.K2_SetTimerDelegate` (`|CreateDelegate` :!event `OnAttackCooldownEnd`) (`self.AttackCooldown`))
  (set `self.AttackOnCooldown` true))

(fn `StopAnimation`
  (`SkeletalMeshComponent.Stop` (`self.Mesh`))
  (set `self.PlayingAnimation` ""))

(fn `TryAttack`
  (if (`/Game/Content/Game/HealthEffectSystem/Blueprints/BP_StatusEffectComponent.bCanAct` (`self.StatusComponent`))
    (if (not (`self.AttackOnCooldown`))
      (`self.OnAttack`)
      (`self.StartAttackCooldown`))))

(fn `UserConstructionScript`)