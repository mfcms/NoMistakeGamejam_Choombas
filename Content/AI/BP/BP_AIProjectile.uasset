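; AI projectile actor that flies in a straight line toward a target or given destination.
; InitProjectile takes the target actor's current location when valid, otherwise the passed destination, and sets the ProjectileMovement velocity along that direction at Speed, with no homing afterward.
; Overlapping the player pawn prints a debug hit message and destroys the projectile, applying no damage; any blocking hit also destroys it.
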(event `self.ReceiveBeginPlay`)

(event `self.ReceiveActorBeginOverlap`
  (params (OtherActor :type "Actor Object Reference"))
  (if (== OtherActor (`GameplayStatics.GetPlayerPawn` 0))
    (`KismetSystemLibrary.PrintString` "PLAYER HIT")
    (`self.K2_DestroyActor`)))

(event `self.ReceiveHit`
  (params (MyComp :type "PrimitiveComponent Object Reference") (Other :type "Actor Object Reference") (OtherComp :type "PrimitiveComponent Object Reference") (bSelfMoved :type Boolean) (HitLocation :type "Vector Structure") (HitNormal :type "Vector Structure") (NormalImpulse :type "Vector Structure") (Hit :type "HitResult Structure (by ref)"))
  (`self.K2_DestroyActor`))

(fn `InitProjectile`
  (params (TargetActor :type "Actor Object Reference") (Destination :type "Vector Structure"))
  (bind _target (`self.Target`))
  (set `self.Target` TargetActor)
  (set `self.Destination` Destination)
  (if (`KismetSystemLibrary.IsValid` _target)
    (bind _output_get (set `self.Destination` (`self.K2_GetActorLocation` _target)))
    (set `self.Destination` (`KismetMathLibrary.MakeVector` (.x _output_get) (.y _output_get) (.z _output_get))))
  (set `MovementComponent.Velocity` (* (`KismetMathLibrary.Normal` (- (`self.Destination`) (`self.K2_GetActorLocation`))) (`self.Speed`)) (`self.ProjectileMovement`)))

(fn `UserConstructionScript`)