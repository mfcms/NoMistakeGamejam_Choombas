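; Boss enemy AI that teleports between destructible columns, summoning enemies until no columns remain, then fighting directly.
; OnUpdateAI runs a BossState machine (spawn, teleport, summon, fall, cast), with SwitchState setting IsBusy and delays timed to animation lengths.
; Summoning creates spawners up to MaxSummons; any column's destruction removes it and triggers Fall or Teleport.
; With none left, Cast enables capsule collision and attacks with arrow projectiles aimed at the player.
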(event `OnColumnDestroyed` :!signature `self.OnDestroyed`
  (params (DestroyedActor :type "Actor Object Reference"))
  (bind _asbp_column (cast `/Game/AI/BP_Column` DestroyedActor))
  (`KismetArrayLibrary.Array_RemoveItem` (`self.TeleportColumns`) _asbp_column)
  (if (`NavMovementComponent.IsFalling` (`self.CharacterMovement`))
    (`self.SwitchState` "NewEnumerator2")
    (else
      (`self.SwitchState` "NewEnumerator3"))))

(event `self.ReceiveBeginPlay`
  (`parent.ReceiveBeginPlay`)
  (for _array_element (`self.TeleportColumns`)
    (add `self.OnDestroyed` _array_element (delegate `OnColumnDestroyed`))))

(event `self.OnUpdateAI`
  (bind _teleportcolumns (`self.TeleportColumns`))
  (switch `/Game/AI/E_BossState` (`self.BossState`)
    (:`NewEnumerator5`
      ; None->Spawn
      (`self.SwitchState` "NewEnumerator0")
      (`self.LookAt` (`GameplayStatics.GetPlayerPawn` 0))
      (`self.PlayRandomAnimationFor` "Spawn")
      (`KismetSystemLibrary.Delay` (+ 0.2 (`AnimationAsset.GetPlayLength` (`self.LastStartedAnimation`))))
      (`self.SwitchState` "NewEnumerator3"))
    (:`NewEnumerator8`
      ; Summon
      (`self.PlayRandomAnimationFor` "Summon" true)
      (`self.LookAt` (`GameplayStatics.GetPlayerPawn` 0))
      (`self.SwitchState` "NewEnumerator1" false))
    (:`NewEnumerator1`
      ; Summoning
      (if (< (`self.SummonsCount`) (`self.MaxSummons`))
        (for _array_element (`self.SpawnEnemyTypes`)
          (bind _returnvalue (`|SpawnActorFromClass` "/Game/Content/Game/Spawn/BP_Spawner.BP_Spawner_C" (`self.GetTransform`) "Undefined" "MultiplyWithRoot" null false self (0.0 0.0 0.0) "NewEnumerator1" 200.0 600.0 (make `FloatInterval` 1.0 3.0) _array_element (`KismetMathLibrary.RandomIntegerInRange` 1 (/ (`self.MaxSummons`) 3)) null))
          (`KismetArrayLibrary.Array_Add` (`self.Spawners`) _returnvalue)
          (set `self.SummonsCount` (+ (`self.SummonsCount`) (`/Game/Content/Game/Spawn/BP_Spawner.MaxEnemiesCount` _returnvalue))))))
    (:`NewEnumerator2`
      ; Fall
      (`KismetArrayLibrary.Array_Clear` (`self.Spawners`))
      (if (not (`NavMovementComponent.IsFalling` (`self.CharacterMovement`)))
        (`self.SwitchState` "NewEnumerator3")))
    (:`NewEnumerator3`
      ; Teleport
      (if (`KismetArrayLibrary.Array_IsEmpty` _teleportcolumns)
        (`self.SwitchState` "NewEnumerator4" false)
        (else
          (bind _output_get (set `self.CurrentColumn` (`KismetArrayLibrary.Array_Random` _teleportcolumns)))
          (`self.LookAt` _output_get)
          (`self.PlayRandomAnimationFor` "Teleport")
          (`self.SwitchState` "NewEnumerator7")
          (`KismetSystemLibrary.Delay` (+ 0.2 (`AnimationAsset.GetPlayLength` (`self.LastStartedAnimation`))))
          (`self.K2_TeleportTo` (`SceneComponent.K2_GetComponentLocation` (`self.FindComponentByTag` _output_get "/Script/Engine.SceneComponent" "TeleportLocation")))
          (`self.SwitchState` "NewEnumerator8" false))))
    (:`NewEnumerator4`
      ; Cast
      (`self.TryAttack`))))

(event `self.OnAttack`
  (`self.Attack`))

(fn `Attack`
  (bind _returnvalue (`self.GetTransform`))
  (if (not (`self.AttackOnCooldown`))
    (`self.PlayRandomAnimationFor` "Attack" false (`self.AttackCooldown`))
    (bind _returnvalue_2 (`|SpawnActorFromClass` "/Game/AI/BP/BP_AIProjectileArrow.BP_AIProjectileArrow_C" _returnvalue "Undefined" "MultiplyWithRoot" null 400.0 null))
    (`self.K2_SetActorRotation` _returnvalue_2 (`KismetMathLibrary.FindLookAtRotation` (.location _returnvalue) (`self.K2_GetActorLocation` (`GameplayStatics.GetPlayerPawn` 0))) false)
    (`/Game/AI/BP/BP_AIProjectile.InitProjectile` _returnvalue_2 (`GameplayStatics.GetPlayerPawn` 0) (0.0 0.0 0.0))))

(fn `LookAt`
  (params (TargetActor :type "Actor Object Reference"))
  (`AIController.K2_SetFocus` (`AIBlueprintHelperLibrary.GetAIController` self) TargetActor)
  (return))

(fn `SwitchState`
  (params (ToState :type "/Game/AI/E_BossState Enum" :default "NewEnumerator5") (SetIsBusy :type Boolean :default true))
  (set `self.BossState` ToState)
  (set `self.IsBusy` SetIsBusy)
  (if (`|EnumEquality` (`self.BossState`) "NewEnumerator4")
    (`PrimitiveComponent.SetCollisionEnabled` (`self.CapsuleComponent`) "QueryAndPhysics")))

(fn `UserConstructionScript`
  (`parent.UserConstructionScript`))