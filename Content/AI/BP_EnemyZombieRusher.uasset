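; Zombie enemy AI variant that walks toward the player and breaks into a rush when within rush distance.
; Each AI update moves to the player pawn while outside attack radius, otherwise tries to attack, as does a successful move.
; An XOR against IsRushing fires only when the rush threshold is crossed, switching desired walk speed on the StatusComponent and the looping Run or Walk animation.
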(event `self.OnUpdateAI`
  (bind _statuscomponent (`self.StatusComponent`))
  (bind _returnvalue (<= (`self.DistanceToPlayer`) (`self.RushDistance`)))
  (if (> (`self.DistanceToPlayer`) (`self.AttackRadius`))
    (`self.OnMoveTo` (0.0 0.0 0.0) (`GameplayStatics.GetPlayerPawn` 0) (`self.WalkToRadius`))
    (if (xor _returnvalue (`self.IsRushing`))
      (bind _speed (`/Game/Content/Game/HealthEffectSystem/Blueprints/BP_StatusEffectComponent.GetConfiguredWalkSpeed` _statuscomponent (`self.MaxSpeed`)))
      (`/Game/Content/Game/HealthEffectSystem/Blueprints/BP_StatusEffectComponent.SetDesiredWalkSpeed` _statuscomponent (`KismetMathLibrary.SelectFloat` (`self.MaxSpeedRush`) _speed _returnvalue))
      (`self.PlayRandomAnimationFor` (`KismetMathLibrary.SelectString` "Run" "Walk" _returnvalue) true)
      (set `self.IsRushing` (not (`self.IsRushing`))))
    (else
      (`self.TryAttack` :!label _label))))

(event `self.OnMoveToSuccess`
  (goto _label))

(event `self.ReceiveBeginPlay`
  (`parent.ReceiveBeginPlay`))

(fn `UserConstructionScript`
  (`parent.UserConstructionScript`))