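; BP_InputJuggler is a test Blueprint that randomly rebinds the IA_Print1 Enhanced Input action each time it fires.
; On each trigger it removes IMC_Test and the previous generated context, then constructs a new Input Mapping Context at runtime.
; It maps the action to a random R, T or Y key, adds the context, stores it for later removal, and prints the new key.
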(event `self.ReceiveBeginPlay`)

(event `self.ReceiveTick`
  (params (DeltaSeconds :type "Float (single-precision)")))

(event `EnhancedInput|/Game/Input/IA_Print1`
  (params (ActionValue :type Boolean) (ElapsedSeconds :type "Float (double-precision)") (TriggeredSeconds :type "Float (double-precision)") (InputAction :type "InputAction Object Reference" :default "/Game/Input/IA_Print1.IA_Print1"))
  (bind _returnvalue (pcsubsystem `EnhancedInputLocalPlayerSubsystem` (`GameplayStatics.GetPlayerController` 0)))
  (:`Triggered`
    (`KismetSystemLibrary.PrintString` "INPUT")
    (`EnhancedInputSubsystemInterface.RemoveMappingContext` _returnvalue "/Game/Input/IMC_Test.IMC_Test" (make `ModifyContextOptions` false true))
    (`EnhancedInputSubsystemInterface.RemoveMappingContext` _returnvalue (`self.OldInputMapping`) (make `ModifyContextOptions` false true))
    (bind _returnvalue_2 (`|GenericCreateObject` "/Script/EnhancedInput.InputMappingContext"))
    (bind _output_get (set `self.NewInputMapping` _returnvalue_2))
    (bind _output_get_2 (set `self.NewKey` (`KismetArrayLibrary.Array_Random` (`|MakeArray` "R" "T" "Y" :!type "Key Structure"))))
    (`InputMappingContext.MapKey` _output_get "/Game/Input/IA_Print1.IA_Print1" _output_get_2)
    (`EnhancedInputSubsystemInterface.AddMappingContext` (pcsubsystem `EnhancedInputLocalPlayerSubsystem` (`GameplayStatics.GetPlayerController` 0)) (`self.NewInputMapping`) 0 (struct))
    (set `self.OldInputMapping` (`self.NewInputMapping`))
    (`KismetSystemLibrary.PrintString` (`KismetStringLibrary.Concat_StrStr` "NewKey: " (`KismetTextLibrary.Conv_TextToString` (`KismetInputLibrary.Key_GetDisplayName` (`self.NewKey`)))))))

(fn `UserConstructionScript`)