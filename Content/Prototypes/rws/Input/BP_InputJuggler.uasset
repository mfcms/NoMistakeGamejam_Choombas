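; Prototype input actor that cycles Enhanced Input mapping contexts for spells at runtime.
; It records the last added context through a subsystem delegate, seeded with IMC_Spells1234 if that is active at BeginPlay.
; IA_Spell01 removes the recorded context, steps a wrapping index through SpellMappings, adds that context and prints its name.
; The other three spell actions are empty.
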(event `self.ReceiveBeginPlay`
  (bind _returnvalue (pcsubsystem `EnhancedInputLocalPlayerSubsystem` (`GameplayStatics.GetPlayerController` 0)))
  (add `EnhancedInputLocalPlayerSubsystem.OnMappingContextAdded` _returnvalue (delegate `On Mapping Context Added`))
  (if (`.ReturnValue` (`EnhancedInputSubsystemInterface.HasMappingContext` _returnvalue "/Game/Prototypes/rws/Input/IMC_Spells1234.IMC_Spells1234"))
    (set `self.OldInputMapping` "/Game/Prototypes/rws/Input/IMC_Spells1234.IMC_Spells1234")))

(event `On Mapping Context Added`
  (params (MappingContext :type "InputMappingContext Object Reference"))
  (set `self.OldInputMapping` MappingContext))

(event `self.ReceiveTick`
  (params (DeltaSeconds :type "Float (single-precision)")))

(event `EnhancedInput|/Game/Prototypes/rws/Input/IA_Spell01`
  (params (ActionValue :type Boolean) (ElapsedSeconds :type "Float (double-precision)") (TriggeredSeconds :type "Float (double-precision)") (InputAction :type "InputAction Object Reference" :default "/Game/Prototypes/rws/Input/IA_Spell01.IA_Spell01"))
  (:`Triggered`
    (`EnhancedInputSubsystemInterface.RemoveMappingContext` (pcsubsystem `EnhancedInputLocalPlayerSubsystem` (`GameplayStatics.GetPlayerController` 0)) (`self.OldInputMapping`) (make `ModifyContextOptions` false true))
    (bind _result (`/Engine/EditorBlueprintResources/StandardMacros.IncrementInt` (`self.SpellMappingIndex`))
      (:`  `
        (bind _output_get (set `self.SpellMappingIndex` (mod _result (`KismetArrayLibrary.Array_Length` (`self.SpellMappings`)))))
        (bind _output (`|GetArrayItem` (`self.SpellMappings`) _output_get))
        (`EnhancedInputSubsystemInterface.AddMappingContext` (pcsubsystem `EnhancedInputLocalPlayerSubsystem` (`GameplayStatics.GetPlayerController` 0)) _output 0 (struct))
        (`KismetSystemLibrary.PrintString` (`KismetStringLibrary.Concat_StrStr` "Mapping: " (`KismetSystemLibrary.GetDisplayName` _output)))))))

(event `EnhancedInput|/Game/Prototypes/rws/Input/IA_Spell02`
  (params (ActionValue :type Boolean) (ElapsedSeconds :type "Float (double-precision)") (TriggeredSeconds :type "Float (double-precision)") (InputAction :type "InputAction Object Reference" :default "/Game/Prototypes/rws/Input/IA_Spell02.IA_Spell02")))

(event `EnhancedInput|/Game/Prototypes/rws/Input/IA_Spell03`
  (params (ActionValue :type Boolean) (ElapsedSeconds :type "Float (double-precision)") (TriggeredSeconds :type "Float (double-precision)") (InputAction :type "InputAction Object Reference" :default "/Game/Prototypes/rws/Input/IA_Spell03.IA_Spell03")))

(event `EnhancedInput|/Game/Prototypes/rws/Input/IA_Spell04`
  (params (ActionValue :type Boolean) (ElapsedSeconds :type "Float (double-precision)") (TriggeredSeconds :type "Float (double-precision)") (InputAction :type "InputAction Object Reference" :default "/Game/Prototypes/rws/Input/IA_Spell04.IA_Spell04")))

(fn `UserConstructionScript`)